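; BP_ItemChest is an interactive, one-time-open chest prop that reveals either a coin or a trap bomb.
; The construction script picks the contents by weighted random roll from the procedural dungeon game instance's seed stream, setting the trap flag and item mesh.
; On interaction, a timeline rotates the lid and moves and spins the item.
; When it finishes, the item hides and a coin burst or explosion particle effect spawns.
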(event EventInteractionIF
  (params (InteractingActor :type Actor%20Object%20Reference))
  (bind _item (Variables|Default|GetItem))
  (bind _returnvalue (Transformation|GetWorldLocation _item))
  (if (not (Variables|Default|GetChestOpen?))
    (Variables|Default|SetChestOpen? true)
    (bind (_direction _open_close _itemlocation _itemrotation) (Timeline|ItemAnimation Play)
      (:Update
        (Transformation|SetRelativeRotation (Variables|Default|GetLid) (Math|Rotator|MakeRotator _open_close 0.0 0.0) false false)
        (Transformation|SetRelativeLocationAndRotation (Variables|Default|GetItemOffset) (Math|Vector|MakeVector 0.0 0.0 _itemlocation) (Math|Rotator|MakeRotator 0.0 0.0 _itemrotation) false false))
      (:Finished
        (Rendering|SetVisibility _item false false)
        (if (Variables|Default|GetIsTrap?)
          (Effects|SpawnEmitteratLocation "/Game/StarterContent/Particles/P_Explosion.P_Explosion" _returnvalue)
          (else
            (Effects|SpawnEmitteratLocation "/Game/Effects/Particles/Meshes/Coins/P_CoinBurst.P_CoinBurst" _returnvalue)))))))

(fn ConstructionScript
  (bind _item (Variables|Default|GetItem))
  (bind _asbp_procedural_dungeon_gi (Utilities|Casting|CastToBP_ProceduralDungeon_GI (Game|GetGameInstance)))
  (if (Class|KismetMathLibrary|RandomBoolwithWeightfromStream (Variables|/Game/Blueprints/ConfigData/GameInstances/BP_ProceduralDungeon_GI.BP_ProceduralDungeon_GI_C|GetSeedStream _asbp_procedural_dungeon_gi) (Variables|Default|GetTrapPercentageWeight))
    (Variables|Default|SetIsTrap? true)
    (Components|StaticMesh|SetStaticMesh _item "/Game/Meshes/Props/Bombs/CartoonBomb.CartoonBomb")
    (else
      (Variables|Default|SetIsTrap? false)
      (Components|StaticMesh|SetStaticMesh _item "/Game/Meshes/Collectables/Valuables/Coins/Coin_01/Coin.Coin"))))