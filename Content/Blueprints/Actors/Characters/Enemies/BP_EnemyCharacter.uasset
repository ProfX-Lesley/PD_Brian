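; Enemy character that roams the level, pursues the player's explorer and restarts MainLevel behind a fade-out when its capture zone touches them.
; Roaming loops between random navigable points, while AI perception switches it to running at the sensed explorer or moving to the last stimulus location.
; The interaction interface acts as a one-time kick: an explosion, an impulse-launched ragdoll, removed capsule and capture zone, and brief slow motion.
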(event OnTargetPerceptionUpdated(AIPerception)
  (params (Actor :type Actor%20Object%20Reference) (Stimulus :type AI%20Stimulus%20Structure))
  (bind _self self)
  (bind _returnvalue (AI|GetAIController _self))
  (bind _asbp_explorer_character (Utilities|Casting|CastToBP_ExplorerCharacter Actor))
  (if (.bsuccessfullysensed Stimulus)
    (AI|Navigation|SimpleMovetoActor _returnvalue _asbp_explorer_character)
    (Variables|/Script/Engine.CharacterMovementComponent|SetMaxWalkSpeed (Variables|Character|GetCharacterMovement) (Variables|Default|GetRunSpeed))
    (else
      (AI|Navigation|MovetoLocation _returnvalue (.stimuluslocation Stimulus) -1.0 true true false true 0))))

(event OnComponentBeginOverlap(EnemyCaptureZone)
  (params (OverlappedComponent :type Primitive%20Component%20Object%20Reference) (OtherActor :type Actor%20Object%20Reference) (OtherComp :type Primitive%20Component%20Object%20Reference) (OtherBodyIndex :type Integer) (bFromSweep :type Boolean) (SweepResult :type Hit%20Result%20Structure%20%28by%20ref%29))
  (Utilities|Casting|CastToBP_ExplorerCharacter OtherActor)
  (CameraFades|StartCameraFade :self (Game|GetPlayerCameraManager 0) :ToAlpha 1.0 :Duration 1.5 :bHoldWhenFinished true)
  (Utilities|FlowControl|Delay 1.5)
  (Game|OpenLevel(byName) "MainLevel"))

(event Custom|Roaming
  (bind _randomlocation (Class|NavigationSystemV1|GetRandomLocationinNavigableRadius (Transformation|GetWorldLocation (Variables|Character|GetMesh)) (Variables|Default|GetRoamingRadius) 0 0))
  (AI|AIMoveTo self _randomlocation 0 1e+02 false
    (:OnSuccess
      _)
    (:OnFail
      _))
  (Utilities|FlowControl|Delay 2.0)
  (CallFunction|Roaming))

(event EventBeginPlay
  (CallFunction|Roaming))

(event EventInteractionIF
  (params (InteractingActor :type Actor%20Object%20Reference))
  (bind _mesh (Variables|Character|GetMesh))
  (Utilities|FlowControl|DoOnce false
    (:Completed
      (Effects|SpawnEmitterAttached "/Game/Effects/Particles/Sprites/Explosion/P_Explosion.P_Explosion" (Variables|Character|GetMesh) "pelvis")
      (Physics|SetSimulatePhysics _mesh true)
      (Collision|SetCollisionProfileName _mesh "Ragdoll" true :!class /Script/Engine.PrimitiveComponent)
      (Physics|AddImpulse _mesh (* (Math|Vector|Normalize (Utilities|Operators|Subtract (Transformation|GetActorLocation) (Transformation|GetActorLocation InteractingActor) (Math|Vector|MakeVector 0.0 0.0 (* (Variables|Default|GetKickHeight) 1e+03)))) (Variables|Default|GetKickForce)) "None" true)
      (Components|DestroyComponent (Variables|Collision|GetCapsuleComponent))
      (Utilities|Time|SetGlobalTimeDilation 0.2)
      (Utilities|FlowControl|Delay 0.2)
      (Utilities|Time|SetGlobalTimeDilation 1.0))))

(fn ConstructionScript)