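; Game Instance that builds a seeded procedural dungeon from random start and extension room classes.
; On initialization it resets state, seeds a random stream (zero means random) and spawns a start room, with a delay before extending for the main menu.
; An extension room spawns at a random collected endpoint, then its collision boxes are checked for overlaps.
; As written, generation places one extension without looping or acting on the overlap result.
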(event EventInitializedDungeonIF
  (CallFunction|VariablesReset)
  (CallFunction|ProcessSeedInput)
  (Utilities|PrintExtensions)
  (if (Variables|Default|GetIsMainMenu?_GI)
    (bind _output_get (Variables|Default|SetBuildDelay 1.0))
    (CallFunction|GenerateStarterRoom)
    (Utilities|FlowControl|Delay _output_get)
    (CallFunction|GenerateExtensionRooms)
    (else
      (Variables|Default|SetBuildDelay 0.01)
      (CallFunction|GenerateStarterRoom)
      (CallFunction|GenerateExtensionRooms))))

(fn ProcessSeedInput
  (bind _seedstream (Variables|Default|GetSeedStream))
  (if (== (Variables|Default|GetLoadingSeed) 0) ; If the user inputted 0 as their\ndesired seed, then it will ignore\nthe input, and the seed will be\nrandomized\n\nIf the user did not input 0,\nthen the inputted number will be\nset as the seed number moving forward
    (Class|KismetMathLibrary|SeedRandomStream _seedstream) ; Similar to a variable Setter, but with\nmore functionality.\nThis sets the random seed to be a\nrandom value.
    (Variables|Default|SetLoadingSeed (.initialseed (Variables|Default|GetSeedStream))) ; Used as a reference of the seed
    (else
      (Math|Random|SetRandomStreamSeed _seedstream (Variables|Default|GetLoadingSeed)) ; Also similar to a variable setter\nwith more functionality\nLooks aat the User's inputted number,\nthen sets it as the random seed
    )))

(fn GenerateStarterRoom
  (bind _returnvalue (Game|SpawnActorfromClass (CallFunction|RandomizeStartRoom) (Variables|Default|GetStartRoomSpawnPoint) "Undefined" "MultiplyWithRoot" 0 0)) ; Spawns in the Starting Room
  (Variables|Default|SetAllEndPoints (Variables|Default|GetAllEndPoints))
  (Utilities|Array|AppendArray (Variables|Default|GetAllEndPoints) (Components|GetChildrenComponents (Variables|/Game/Blueprints/Actors/DungeonRooms/BP_Room_Master.BP_Room_Master_C|GetEndPoints_Grp _returnvalue) false))
  (return))

(fn RandomizeStartRoom
  (bind _startroomclasses (Variables|Default|GetStartRoomClasses))
  (return (Utilities|Array|Get(acopy) _startroomclasses (Math|Random|RandomIntegerinRangefromStream (Variables|Default|GetSeedStream) 0 (- (Utilities|Array|Length _startroomclasses) 1)))))

(fn VariablesReset
  (Utilities|Array|Clear (Variables|Default|GetAllEndPoints))
  (Variables|Default|SetExtensions (- (Variables|Default|GetTotalRooms) 1))
  (Variables|Default|SetCurrentRoom 0)
  (Variables|Default|SetStartRoomSpawnPoint ""))

(fn GenerateExtensionRooms
  (if (> (Variables|Default|GetExtensions) 0)
    (bind _chosenendpoint (Utilities|RandomEndpointSelect (Variables|Default|GetAllEndPoints)))
    (bind (_chosenextensionclass _chosenextensionclassindex _endpointtransform) (Utilities|EndPointCheck _chosenendpoint)
      (:ValidEndpoint
        (bind _returnvalue (Game|SpawnActorfromClass _chosenextensionclass _endpointtransform "Undefined" "MultiplyWithRoot" 0 0))
        (Utilities|RoomOverlapCheck _returnvalue)))))